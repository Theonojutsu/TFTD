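; Player board pawn that builds a hex grid, bench row and gold stacks, and lets the player drag heroes between tiles.
; The construction script builds instanced meshes with per-instance colour data, records hex and bench tiles, and positions the camera.
; Mouse input feeds event dispatchers; cursor traces pick heroes, and nearest-tile lookups against occupancy arrays choose grab, release or swap.
; Tick makes the held hero follow the cursor or snaps it onto its tile.
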(fn ConstructionScript
  (CallFunction|UpdateHexGrid))

(fn BuildHexRow
  (params (NumberOfRow :type Integer) (PlaceLocation :type Vector))
  (bind _tilehex (Variables|Board|GetTileHex))
  (bind _spacinghard (Variables|Board|GetSpacingHard))
  (bind _scale (Variables|GridProperty|GetScale))
  ;[0 0 0 0.5 50] BuildRow
  (for _index (range 0 (- (Variables|GridProperty|GetRowLength) 1))
    (bind _returnvalue (Components|InstancedStaticMesh|AddInstance (Variables|Board|GetTileHex) (Math|Transform|MakeTransform (Math|Vector|MakeVector (+ (* NumberOfRow (Variables|Board|GetHexOffset) (Math|Trig|Sin(Degrees) 6e+01) _spacinghard) (.x PlaceLocation)) (+ (.y PlaceLocation) (* _spacinghard (Variables|Board|GetHexOffset) _index)) (.z PlaceLocation)) "0, 0, 0" (Math|Vector|MakeVector _scale _scale 1.0)) true))
    (CallFunction|UpdateColor&Opacity _returnvalue _tilehex (Variables|GridProperty|GetColorHex))
    (Utilities|Array|Add (Variables|Board|GetAllTiles) (Utilities|Struct|MakeStruct_Tiles _returnvalue (.location (.OutInstanceTransform (Components|InstancedStaticMesh|GetInstanceTransform _tilehex _returnvalue true)))))))

(fn GetOffsetLocation
  (bind _returnvalue (Transformation|GetActorLocation))
  (return (Math|Vector|MakeVector (.x _returnvalue) (+ (.y _returnvalue) (* (* (Variables|Board|GetHexOffset) (Variables|Board|GetSpacingHard)) (Math|Trig|Cos(Degrees) 6e+01))) (.z _returnvalue))))

(fn FindOffset
  (params (InstancedMesh :type Static%20Mesh%20Component%20Object%20Reference))
  (return (* (Variables|GridProperty|GetScale) (.y (.Max (Components|StaticMesh|GetLocalBounds InstancedMesh))) 2.0)))

(fn UpdateColor&Opacity
  (params (InstanceIndex :type Integer) (InstancedMesh :type Instanced%20Static%20Mesh%20Component%20Object%20Reference) (Color :type Linear%20Color%20Structure))
  (bind _output_get (Variables|GridProperty|SetColorHex Color))
  (Components|InstancedStaticMesh|SetCustomDataValue InstancedMesh InstanceIndex 0 (.r _output_get) false)
  (Components|InstancedStaticMesh|SetCustomDataValue InstancedMesh InstanceIndex 1 (.g _output_get) false)
  (Components|InstancedStaticMesh|SetCustomDataValue InstancedMesh InstanceIndex 2 (.b _output_get) false)
  (Components|InstancedStaticMesh|SetCustomDataValue InstancedMesh InstanceIndex 3 (.a _output_get) false))

(fn PlaceHeroonTile&UpdateOccupy
  (params (Hero :type Actor%20Object%20Reference) (OccupiedTileArray :type Array%20of%20Struct%20Occupied%20Tiles%20Structures) (Destination :type Vector))
  (bind _nearesttile (Variables|Board|GetNearestTile))
  ;[0 0 0 0.5 50] Place Hero on targeted Tile
  (Transformation|SetActorLocation Hero Destination false true)
  ;[0 0 0 0.5 50] Add Hero and its tile to Occupied tile array
  (Utilities|Array|Add OccupiedTileArray (Utilities|Struct|MakeStruct_OccupiedTiles (Variables|Board|GetNearestTile) Hero))
  ;[0 0 0 0.5 50] If "nearest tile" is an empty bench tile, remove it from it & add it to occupied one
  (if (Utilities|Array|ContainsItem (Variables|Board|GetEmptyBenchTiles) (Utilities|Struct|MakeStruct_Tiles (.index _nearesttile) (.location _nearesttile))) ; Does the tile is a bench tile ?
    (Utilities|Array|RemoveItem (Variables|Board|GetEmptyBenchTiles) (Utilities|Struct|MakeStruct_Tiles (.index _nearesttile) (.location _nearesttile)))
    (Utilities|Array|Add (Variables|Board|GetOccupiedBenchTiles) (Utilities|Struct|MakeStruct_OccupiedTiles (Utilities|Struct|MakeStruct_Tiles (.index _nearesttile) (.location _nearesttile)) Hero))
    (return)))

(fn GetOwnPlayerController
  (return 0))

(fn GetLocationUnderCursor
  (bind _array (Utilities|Array|MakeArray "ObjectTypeQuery1" "ObjectTypeQuery7" "ObjectTypeQuery8" "ObjectTypeQuery3"))
  (bind _player_controller_owner (Variables|PlaceHero|GetPlayer%20Controller%20Owner))
  (bind _hitresult (Class|PlayerController|GetHitResultUnderCursorforObjects _player_controller_owner _array true))
  (bind (_bblockinghit _binitialoverlap _time _distance _location _impactpoint _normal _impactnormal _physmat _hitactor) (Collision|BreakHitResult _hitresult))
  (return _bblockinghit _impactpoint _hitactor))

(fn GetImpactLocation
  (bind _player_controller_owner (Variables|PlaceHero|GetPlayer%20Controller%20Owner)
    (:then
      (return (.x (.ImpactPoint (Collision|BreakHitResult (.HitResult (Game|Player|GetHitResultUnderCursorbyChannel _player_controller_owner "TraceTypeQuery1" true))))) (.y (.ImpactPoint (Collision|BreakHitResult (.HitResult (Game|Player|GetHitResultUnderCursorbyChannel _player_controller_owner "TraceTypeQuery1" true)))))))
    (:else)))

(fn SetCamLocation
  (bind _rowlength (Variables|GridProperty|GetRowLength))
  (bind _returnvalue (Math|Conversions|ToFloat(Integer) _rowlength))
  (bind _returnvalue_2 (/ _returnvalue 2.0))
  (bind _returnvalue_3 (Math|Float|Truncate _returnvalue_2))
  (Variables|Board|SetHalfIndex _returnvalue_3)
  (if (Math|Float|NearlyEqual(Float) (- _returnvalue_2 _returnvalue_3) 0.0 0.0001)
    (Transformation|SetRelativeLocation (Variables|Board|GetCamera) (Math|Vector|MakeVector (Variables|GridProperty|GetCamX) (+ (/ (- (.y (.location (.OutInstanceTransform (Components|InstancedStaticMesh|GetInstanceTransform (Variables|Board|GetTileHex) (+ (Variables|Board|GetHalfIndex) 1) true)))) (.y (.location (.OutInstanceTransform (Components|InstancedStaticMesh|GetInstanceTransform (Variables|Board|GetTileHex) (Variables|Board|GetHalfIndex) true))))) 1.5) (.y (.location (.OutInstanceTransform (Components|InstancedStaticMesh|GetInstanceTransform (Variables|Board|GetTileHex) (- (Variables|Board|GetHalfIndex) 1) false))))) (Variables|GridProperty|GetCamZ)) false true)
    (else
      (Transformation|SetRelativeLocation (Variables|Board|GetCamera) (Math|Vector|MakeVector (Variables|GridProperty|GetCamX) (.y (.location (.OutInstanceTransform (Components|InstancedStaticMesh|GetInstanceTransform (Variables|Board|GetTileHex) (Variables|Board|GetHalfIndex) false)))) (Variables|GridProperty|GetCamZ)) false true))))

(fn UpdateHexGrid
  (bind _tilehex (Variables|Board|GetTileHex))
  (bind _tilebench (Variables|Board|GetTileBench))
  (bind _tilegoldstack (Variables|Board|GetTileGoldStack))
  (Components|InstancedStaticMesh|ClearInstances (Variables|Board|GetTileHex))
  (CallFunction|FindSpacing)
  (Utilities|FlowControl|Sequence
    (:then_0
      (Components|StaticMesh|SetStaticMesh _tilehex (Variables|Board|GetSelectedHexMesh))
      (Rendering|Material|SetMaterial _tilehex 0 (Variables|GridProperty|GetHex%20Material))
      (Class|InstancedStaticMeshComponent|SetNumCustomDataFloats (Variables|Board|GetTileHex) 4)
      (bind _returnvalue (CallFunction|FindOffset (Variables|Board|GetTileHex)))
      (Variables|Board|SetHexOffset _returnvalue)
      (for _index (range 0 (- (Variables|GridProperty|GetNumRow) 1))
        (CallFunction|BuildHexRow _index (Math|Vector|SelectVector (Transformation|GetActorLocation) (CallFunction|GetOffsetLocation) (!= (Math|Integer|%(Integer) _index 2) 0))))
      (Variables|Board|SetLastIndexHex (+ _index 1)))
    (:then_1
      (Components|StaticMesh|SetStaticMesh _tilebench (Variables|Board|GetSelectedBenchMesh))
      (Rendering|Material|SetMaterial _tilebench 0 (Variables|GridProperty|GetBench%20Material))
      (Class|InstancedStaticMeshComponent|SetNumCustomDataFloats (Variables|Board|GetTileBench) 4)
      (bind _returnvalue_2 (CallFunction|FindOffset (Variables|Board|GetTileBench)))
      (Variables|Board|SetBenchPlatformOffset _returnvalue_2)
      (for _index_2 (range 0 (- (Math|Float|Round (* (Variables|GridProperty|GetRowLength) (/ 1e+01 7.0))) 1))
        (CallFunction|BuildBenchRow _index_2)))
    (:then_2
      (Components|StaticMesh|SetStaticMesh _tilegoldstack (Variables|Board|GetSelectedGoldStackMesh))
      (Rendering|Material|SetMaterial _tilegoldstack 0 (Variables|GridProperty|GetBench%20Material))
      (Class|InstancedStaticMeshComponent|SetNumCustomDataFloats (Variables|Board|GetTileGoldStack) 4)
      (bind _returnvalue_3 (CallFunction|FindOffset (Variables|Board|GetTileGoldStack)))
      (Variables|Board|SetGlodStackOffset _returnvalue_3)
      (for _index_3 (range 0 (- (Variables|GridProperty|GetGoldStackNumber) 1))
        (CallFunction|BuildGoldStack _index_3)))
    (:then_3
      (CallFunction|SetCamLocation))))

(fn BuildBenchRow
  (params (NumberInRow :type Integer))
  (bind _scene (Variables|Board|GetScene))
  (bind _tilebench (Variables|Board|GetTileBench))
  (bind _scale (Variables|GridProperty|GetScale))
  (bind _benchplatformoffset (Variables|Board|GetBenchPlatformOffset))
  (bind _returnvalue (Transformation|GetWorldLocation _scene))
  (bind _returnvalue_2 (Components|InstancedStaticMesh|AddInstance (Variables|Board|GetTileBench) (Math|Transform|MakeTransform (Math|Vector|MakeVector (- (.x _returnvalue) (* (Variables|Board|GetBenchPlatformOffset) (Variables|Board|GetSpacingHard) 1.25)) (+ (- (.y _returnvalue) (Variables|Board|GetBenchPlatformOffset)) (* NumberInRow (Variables|Board|GetSpacingHard) _benchplatformoffset) (/ _benchplatformoffset 2.0)) (.z _returnvalue)) "0, 0, 0" (Math|Vector|MakeVector _scale _scale 1.0)) true))
  (CallFunction|UpdateColor&Opacity _returnvalue_2 _tilebench (Variables|GridProperty|GetColorHex))
  (Utilities|Array|Add (Variables|Board|GetAllTiles) (Utilities|Struct|MakeStruct_Tiles (+ _returnvalue_2 (Variables|Board|GetLastIndexHex)) (.location (.OutInstanceTransform (Components|InstancedStaticMesh|GetInstanceTransform _tilebench _returnvalue_2 true)))))
  (Utilities|Array|Add (Variables|Board|GetEmptyBenchTiles) (Utilities|Struct|MakeStruct_Tiles (+ _returnvalue_2 (Variables|Board|GetLastIndexHex)) (.location (.OutInstanceTransform (Components|InstancedStaticMesh|GetInstanceTransform _tilebench _returnvalue_2 true))))))

(fn FindSpacing
  (Variables|Board|SetSpacingHard (+ 1.0 (/ (Variables|GridProperty|GetSpacing) 1e+02))))

(fn CheckHitActorType
  (bind (_hit _location _hitactor) (CallFunction|GetLocationUnderCursor))
  (bind _returnvalue (Utilities|GetClass _hitactor))
  (if _hit
    (Variables|PlaceHero|SetCachedDestination _location)
    (if (== _hitactor self)
      (Variables|PlaceHero|SetObjectTypes "NewEnumerator1")
      (elif (and (Utilities|ClassIsChildOf _returnvalue "/Script/Engine.Pawn") (!= _returnvalue (Utilities|GetClass self)))
        (Variables|PlaceHero|SetObjectTypes "NewEnumerator0")
        (else
          (Variables|PlaceHero|SetObjectTypes "NewEnumerator2"))))
    (return _hitactor (Variables|PlaceHero|GetObjectTypes) (Variables|PlaceHero|GetCachedDestination))))

(fn GetFollowLocation
  (bind (_impactpoint_x _impactpoint_y) (CallFunction|GetImpactLocation))
  (return (Math|Interpolation|VInterpTo (Transformation|GetActorLocation (Variables|PlaceHero|GetHero)) (Math|Vector|MakeVector _impactpoint_x _impactpoint_y (Variables|PlaceHero|GetZHoveringHero)) (Utilities|Time|GetWorldDeltaSeconds) 2e+01)))

(fn IsHexOccupied?
  (params (HeroXY :type Vector) (NearestTile :type Struct%20Tiles%20Structure%20%28by%20ref%29))
  (bind _location (Utilities|Struct|BreakStruct_Tiles NearestTile))
  (bind (_x _y) (Math|Vector|BreakVector HeroXY))
  (return (Utilities|Operators|EqualEqual (Math|Vector2D|MakeVector2D _x _y) (Math|Vector2D|MakeVector2D (.x _location) (.y _location)) 1.0)))

(fn BuildGoldStack
  (params (InputPin :type Integer))
  (bind _returnvalue (Transformation|GetActorLocation))
  (bind _scale (Variables|GridProperty|GetScale))
  (bind _returnvalue_2 (Components|InstancedStaticMesh|AddInstance (Variables|Board|GetTileGoldStack) (Math|Transform|MakeTransform (Math|Vector|MakeVector (+ (* InputPin (Variables|Board|GetGlodStackOffset) (Variables|Board|GetSpacingHard)) (+ (.x _returnvalue) (/ (Variables|Board|GetHexOffset) 2.0))) (- (.y _returnvalue) (* (Variables|Board|GetHexOffset) 1.25)) (.z _returnvalue)) "0, 0, 0" (Math|Vector|MakeVector _scale _scale 1.0)) true))
  (CallFunction|UpdateColor&Opacity _returnvalue_2 (Variables|Board|GetTileGoldStack) (Variables|GridProperty|GetColorHex)))

(fn RemovefromOccupied
  (params (Hero%20on%20Tile :type Actor%20Object%20Reference))
  (bind _nearesttile (Variables|Board|GetNearestTile))
  ;[0 0 0 0.5] If "nearest tile" is an occupied bench tile, remove it from it & add it to empty one
  (Utilities|Array|RemoveItem (Variables|Board|GetOccupiedTiles) (Variables|Board|GetOccupiedTile))
  (if (Utilities|Array|ContainsItem (Variables|Board|GetOccupiedBenchTiles) (Utilities|Struct|MakeStruct_OccupiedTiles (Utilities|Struct|MakeStruct_Tiles (.index _nearesttile) (.location _nearesttile)) Hero%20on%20Tile)) ; Does the tile is a bench tile ?
    (Utilities|Array|RemoveItem (Variables|Board|GetOccupiedBenchTiles) (Utilities|Struct|MakeStruct_OccupiedTiles (Utilities|Struct|MakeStruct_Tiles (.index _nearesttile) (.location _nearesttile)) Hero%20on%20Tile))
    (Utilities|Array|Add (Variables|Board|GetEmptyBenchTiles) (Utilities|Struct|MakeStruct_Tiles (.index _nearesttile) (.location _nearesttile)))))

(fn FindNearestTile&CheckifOccupied
  (params (HeroLocation :type Vector) (NearestTileArray :type Array%20of%20Struct%20Tiles%20Structures) (OccupiedTileArray :type Array%20of%20Struct%20Occupied%20Tiles%20Structures))
  ;[0 0 0 0.5 50] Find Nearest Tile
  (Variables|PlaceHero|SetCurrentDistance 1e+12)
  (for _array_element NearestTileArray
    (if (< (Math|Vector|Distance(Vector) (.location _array_element) HeroLocation) (Variables|PlaceHero|GetCurrentDistance))
      (Variables|PlaceHero|SetCurrentDistance (Math|Vector|Distance(Vector) (.location _array_element) HeroLocation))
      (Variables|Board|SetNearestTile (Utilities|Struct|MakeStruct_Tiles (.index _array_element) (.location _array_element)))))
  ;[0 0 0 0.5 50] Check if tile is occupied or not
  (Variables|PlaceHero|SetIsOccupied false)
  (bind _array_element_2 (Utilities|Array|ForEachLoopwithBreak OccupiedTileArray :!label _label)
    (:LoopBody
      (if (CallFunction|IsHexOccupied? (.location (.tiledata _array_element_2)) (Variables|Board|GetNearestTile))
        (Variables|PlaceHero|SetIsOccupied true)
        (Variables|Board|SetOccupiedTile (Utilities|Struct|MakeStruct_OccupiedTiles (Utilities|Struct|MakeStruct_Tiles (.index (.tiledata _array_element_2)) (.location (.tiledata _array_element_2))) (.heroontile _array_element_2)))
        (goto _label Break)))
    (:Completed
      (return))))

(fn UpdateGrabConditions
  (params (Hero :type Actor%20Object%20Reference) (Has%20to%20be%20released%20? :type Boolean))
  (Collision|SetActorEnableCollision Hero Has%20to%20be%20released%20?)
  (Variables|/Script/Engine.PlayerController|SetbShowMouseCursor (Variables|PlaceHero|GetPlayer%20Controller%20Owner) Has%20to%20be%20released%20?)
  (Variables|PlaceHero|SetHeroGrabbed (not Has%20to%20be%20released%20?))
  (return))

(fn TargetedTileLocation
  (bind _nearesttile (Variables|Board|GetNearestTile))
  (return (Math|Vector|MakeVector (.x (.location _nearesttile)) (.y (.location _nearesttile)) (+ (.z (.location _nearesttile)) 88.0))))

(event Input|EnhancedActionEvents|EnhancedInputActionIA_LeftClick
  (params (ActionValue :type Boolean) (ElapsedSeconds :type Float%20%28double-precision%29) (TriggeredSeconds :type Float%20%28double-precision%29) (InputAction :type Input%20Action%20Object%20Reference :default "/Game/Board/Input/Actions/IA_LeftClick.IA_LeftClick"))
  ;[0 0 0 0.5 50] Call Mouse Events
  (:Started
    (Default|CallOnLeftClickStarted))
  (:Completed
    (if (> ElapsedSeconds 0.1)
      (Default|CallOnLeftClickCompleted))))

(event Input|EnhancedActionEvents|EnhancedInputActionIA_RightClick
  (params (ActionValue :type Boolean) (ElapsedSeconds :type Float%20%28double-precision%29) (TriggeredSeconds :type Float%20%28double-precision%29) (InputAction :type Input%20Action%20Object%20Reference :default "/Game/Board/Input/Actions/IA_RightClick.IA_RightClick"))
  ;[0 0 0 0.5 50] Call Mouse Events
  (:Started
    (Default|CallOnRightClickStarted)))

(event Input|EnhancedActionEvents|EnhancedInputActionIA_MouseXY
  (params (ActionValue :type Vector%202D%20Structure) (ElapsedSeconds :type Float%20%28double-precision%29) (TriggeredSeconds :type Float%20%28double-precision%29) (InputAction :type Input%20Action%20Object%20Reference :default "/Game/Board/Input/Actions/IA_MouseXY.IA_MouseXY"))
  ;[0 0 0 0.5 50] Call Mouse Events
  (Variables|PlaceHero|SetMousePos ActionValue))

(event EventControllerChanged
  (params (OldController :type Controller%20Object%20Reference) (NewController :type Controller%20Object%20Reference))
  ;[0 0 0 0.5 50] On Possessed
  (Utilities|FlowControl|Sequence
    (:then_0
      ;[0 0 0 1 50] Add IMC
      (bind _output_get (Variables|PlaceHero|SetPlayer%20Controller%20Owner (Game|GetPlayerController 0)))
      (Utilities|IsValid (PlayerController|LocalPlayerSubsystems|GetEnhancedInputLocalPlayerSubsystem _output_get)
        (:Is%20Valid
          (Input|AddMappingContext (PlayerController|LocalPlayerSubsystems|GetEnhancedInputLocalPlayerSubsystem _output_get) "/Game/Board/Input/IMC_GridContext.IMC_GridContext" 0 (Utilities|Struct|MakeModifyContextOptions true false false)))))
    (:then_1
      ;[0 0 0 0.5 50] Bind to Click Events
      (EventDispatchers|BindEventtoOnLeftClickStarted (EventDispatchers|CreateEvent :!event Custom|TryGrab))
      (EventDispatchers|BindEventtoOnLeftClickCompleted (EventDispatchers|CreateEvent :!event Custom|Stop%20Grab))
      (EventDispatchers|BindEventtoOnRightClickStarted (EventDispatchers|CreateEvent :!event Custom|Move))
      (EventDispatchers|BindEventtoOnTick (EventDispatchers|CreateEvent :!event Custom|OnTick)))
    (:then_2
      ;[0 0 0 0.5 50] Set up variables
      (Variables|PlaceHero|SetZHoveringHero (+ (.z (Transformation|GetActorLocation)) 1.5e+02)))
    (:then_3)))

(event Custom|OnTick
  ;[0 0 0 0.5 50] Grab / Release Hero = Follow / Unfollow cursor
  (bind _hero (Variables|PlaceHero|GetHero)
    (:then
      (switch Utilities|FlowControl|Switch|SwitchonE_ClickResponses (Variables|PlaceHero|GetClickResponse)
        (:NewEnumerator0
          (Transformation|SetActorLocation _hero (CallFunction|GetFollowLocation) false true))
        (:NewEnumerator1
          (CallFunction|PlaceHeroonTile&UpdateOccupy (Variables|PlaceHero|GetHero) (Variables|Board|GetOccupiedTiles) (CallFunction|TargetedTileLocation))
          (Variables|PlaceHero|SetHero 0))
        (:NewEnumerator2
          (CallFunction|PlaceHeroonTile&UpdateOccupy (Variables|PlaceHero|GetHero) (Variables|Board|GetOccupiedTiles) (CallFunction|TargetedTileLocation))
          (bind _output_get (Variables|PlaceHero|SetHero (.heroontile (Variables|Board|GetOccupiedTile))))
          (CallFunction|UpdateGrabConditions _output_get false)
          (Variables|PlaceHero|SetClickResponse "NewEnumerator0"))))
    (:else)))

(event Custom|FindNearestHex
  (params (Location :type Vector))
  ;[0 0 0 0.5 50] Find Nearest Place & Check if tile is empty
  (CallFunction|FindNearestTile&CheckifOccupied Location (Variables|Board|GetAllTiles) (Variables|Board|GetOccupiedTiles))
  (CallFunction|ToggleGrab/Release (Variables|PlaceHero|GetIsOccupied)))

(event Custom|ToggleGrab/Release
  (params (Is%20Place%20Occupied :type Boolean))
  ;[0 0 0 0.5 50] Grab / Release Hero = Follow / Unfollow cursor
  (if Is%20Place%20Occupied
    (CallFunction|RemovefromOccupied (Variables|PlaceHero|GetHero))
    (if (!= (.heroontile (Variables|Board|GetOccupiedTile)) (Variables|PlaceHero|GetHero)) ; Is clicked Hero not the \n"Hero" ?
      (Variables|PlaceHero|SetClickResponse "NewEnumerator2")
      (else
        (Variables|PlaceHero|SetClickResponse "NewEnumerator0")))
    (elif (Variables|PlaceHero|GetHeroGrabbed)
      (Variables|PlaceHero|SetClickResponse "NewEnumerator0")
      (else
        (Variables|PlaceHero|SetClickResponse "NewEnumerator1")))))

(event Custom|Stop%20Grab
  ;[0 0 0 0.5 50] Check HitObject type
  (bind _objecttypes (CallFunction|CheckHitActorType))
  (switch Utilities|FlowControl|Switch|SwitchonE_HitTypes _objecttypes
    (:NewEnumerator0
      _)
    (:NewEnumerator1
      _))
  (if (Variables|PlaceHero|GetHeroGrabbed)
    (bind _hero (Variables|PlaceHero|GetHero)
      (:then
        (CallFunction|UpdateGrabConditions _hero true)
        (CallFunction|FindNearestHex (Transformation|GetActorLocation (Variables|PlaceHero|GetHero))))
      (:else))))

(event Custom|TryGrab
  ;[0 0 0 0.5 50] Check HitObject type
  (bind (_hitactor _objecttypes) (CallFunction|CheckHitActorType))
  (switch Utilities|FlowControl|Switch|SwitchonE_HitTypes _objecttypes
    (:NewEnumerator0
      (if (Variables|PlaceHero|GetHeroGrabbed)
        (bind _hero (Variables|PlaceHero|GetHero :!label _label)
          (:then
            (CallFunction|UpdateGrabConditions _hero true))
          (:else))
        (else
          (bind _output_get (Variables|PlaceHero|SetHero _hitactor))
          (CallFunction|UpdateGrabConditions _output_get false)))
      (CallFunction|FindNearestHex (Transformation|GetActorLocation (Variables|PlaceHero|GetHero))))
    (:NewEnumerator1
      (if (Variables|PlaceHero|GetHeroGrabbed)
        (goto _label)))))

(event EventTick
  (params (DeltaSeconds :type Float%20%28single-precision%29))
  (Default|CallOnTick))

(event Custom|Move
  ;[0 0 0 0.5 50] Move around
  (if (not (Variables|PlaceHero|GetHeroGrabbed))
    (bind (_hitactor _objecttypes _cacheddestination) (CallFunction|CheckHitActorType))
    (switch Utilities|FlowControl|Switch|SwitchonE_HitTypes _objecttypes
      (:NewEnumerator1
        _)
      (:NewEnumerator2
        _))
    (Niagara|SpawnSystematLocation (Variables|PlaceHero|GetFXCursor) _cacheddestination)))