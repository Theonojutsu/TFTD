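; Hex board actor that builds a tile grid and snaps pawns to the nearest hex.
; The construction script lays out staggered rows of instanced meshes, stores color and opacity in per-instance custom data, caches hex locations and positions the camera from the first row's midpoint.
; FindNearestHex linearly searches that cache, then teleports the pawn above the closest tile.
; Occupancy tracking and pawn-swap logic exists but is disconnected.
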(event Custom|Place/ReplacePawn
  ;[0 0 0 0.5 50] Place actor on grid
  (CallFunction|SetCurrentPawnonHex))

(event EventFindNearestHex
  (params (Pawn :type Actor%20Object%20Reference) (PawnLocation :type Vector :default "0, 0, 0"))
  ;[0 0 0 0.5 50] Place actor on grid
  (Variables|Grid|SetPawn Pawn)
  (Variables|Grid|SetPawn%20Location PawnLocation)
  (Variables|Grid|SetCurrentDistance 1e+12)
  (for _array_element (Variables|Grid|GetNearestHexes)
    (if (< (Math|Vector|Distance(Vector) (.location _array_element) (Variables|Grid|GetPawn%20Location)) (Variables|Grid|GetCurrentDistance))
      (Variables|Grid|SetCurrentDistance (Math|Vector|Distance(Vector) (.location _array_element) (Variables|Grid|GetPawn%20Location)))
      (Variables|Grid|SetNearestHex (Utilities|Struct|MakeStruct_Hexes (.index _array_element) (.location _array_element)))))
  (CallFunction|Place/ReplacePawn))

(fn ConstructionScript
  (bind _rowlength (Variables|GridProperty|GetRowLength))
  (bind _tilemesh (Variables|Grid|GetTileMesh))
  (bind _returnvalue (Math|Conversions|ToFloat(Integer) _rowlength))
  (bind _returnvalue_2 (/ _returnvalue 2.0))
  (bind _returnvalue_3 (Math|Float|Truncate _returnvalue_2))
  (Components|InstancedStaticMesh|ClearInstances (Variables|Grid|GetTileMesh))
  (Components|StaticMesh|SetStaticMesh _tilemesh (Variables|Grid|GetSelectedMesh))
  (Rendering|Material|SetMaterial _tilemesh 0 (Variables|GridProperty|GetMaterial))
  (Class|InstancedStaticMeshComponent|SetNumCustomDataFloats (Variables|Grid|GetTileMesh) 4)
  (CallFunction|FindOffset)
  (for _index (range 0 (- (Variables|GridProperty|GetNumRow) 1))
    (CallFunction|BuildRow _index (Math|Vector|SelectVector (Transformation|GetActorLocation) (CallFunction|GetOffsetLocation) (== (Math|Integer|%(Integer) _index 2) 0))))
  (Variables|Grid|SetHalfIndex _returnvalue_3)
  (if (Math|Float|NearlyEqual(Float) (- _returnvalue_2 _returnvalue_3) 0.0 0.0001)
    (Transformation|SetRelativeLocation (Variables|Default|GetCamera) (Math|Vector|MakeVector -5e+02 (+ (/ (- (.y (.location (.OutInstanceTransform (Components|InstancedStaticMesh|GetInstanceTransform (Variables|Grid|GetTileMesh) (+ (Variables|Grid|GetHalfIndex) 1) true)))) (.y (.location (.OutInstanceTransform (Components|InstancedStaticMesh|GetInstanceTransform (Variables|Grid|GetTileMesh) (Variables|Grid|GetHalfIndex) true))))) 2.0) (.y (.location (.OutInstanceTransform (Components|InstancedStaticMesh|GetInstanceTransform (Variables|Grid|GetTileMesh) (- (Variables|Grid|GetHalfIndex) 1) false))))) 1.4e+03) false true)
    (else
      (Transformation|SetRelativeLocation (Variables|Default|GetCamera) (Math|Vector|MakeVector 0.0 (.y (.location (.OutInstanceTransform (Components|InstancedStaticMesh|GetInstanceTransform (Variables|Grid|GetTileMesh) (Variables|Grid|GetHalfIndex) false)))) 1.4e+03) false true))))

(fn BuildRow
  (params (NumberOfRow :type Integer) (PlaceLocation :type Vector))
  (bind _scale (Variables|GridProperty|GetScale))
  ;[0.15 0.15 0.15 0.5] BuildRow
  (for _index (range 0 (- (Variables|GridProperty|GetRowLength) 1))
    (bind _returnvalue (Components|InstancedStaticMesh|AddInstance (Variables|Grid|GetTileMesh) (Math|Transform|MakeTransform (Math|Vector|MakeVector (+ (* NumberOfRow (Variables|Grid|GetOffset) (Variables|Grid|GetSpacing) (Math|Trig|Sin(Degrees) 6e+01)) (.x PlaceLocation)) (+ (.y PlaceLocation) (* _index (Variables|Grid|GetOffset) (Variables|Grid|GetSpacing))) (.z PlaceLocation)) "0, 0, 0" (Math|Vector|MakeVector _scale _scale 1.0)) true))
    (CallFunction|UpdateColor&Opacity _returnvalue)
    (Utilities|Array|Add (Variables|Grid|GetNearestHexes) (Utilities|Struct|MakeStruct_Hexes _returnvalue (.location (.OutInstanceTransform (Components|InstancedStaticMesh|GetInstanceTransform (Variables|Grid|GetTileMesh) _returnvalue true)))))))

(fn GetOffsetLocation
  (bind _returnvalue (Transformation|GetActorLocation))
  (return (Math|Vector|MakeVector (.x _returnvalue) (+ (.y _returnvalue) (* (* (Variables|Grid|GetOffset) (Variables|Grid|GetSpacing)) (Math|Trig|Cos(Degrees) 6e+01))) (.z _returnvalue))))

(fn FindOffset
  (Variables|Grid|SetOffset (* (.y (.Max (Components|StaticMesh|GetLocalBounds (Variables|Grid|GetTileMesh)))) (Variables|GridProperty|GetScale)))
  (return))

(fn UpdateColor&Opacity
  (params (InstanceIndex :type Integer))
  (bind _output_get (Variables|GridProperty|SetColor (Variables|GridProperty|GetColor)))
  (Components|InstancedStaticMesh|SetCustomDataValue (Variables|Grid|GetTileMesh) InstanceIndex 0 (.r _output_get) false)
  (Components|InstancedStaticMesh|SetCustomDataValue (Variables|Grid|GetTileMesh) InstanceIndex 1 (.g _output_get) false)
  (Components|InstancedStaticMesh|SetCustomDataValue (Variables|Grid|GetTileMesh) InstanceIndex 2 (.b _output_get) false)
  (Components|InstancedStaticMesh|SetCustomDataValue (Variables|Grid|GetTileMesh) InstanceIndex 3 (.a _output_get) false))

(fn SetCurrentPawnonHex
  (bind _nearesthex (Variables|Grid|GetNearestHex))
  (Transformation|SetActorLocation (Variables|Grid|GetPawn) (Math|Vector|MakeVector (.x (.location _nearesthex)) (.y (.location _nearesthex)) (+ (.z (.location _nearesthex)) 1e+02)) false true))

(fn GetOwnPlayerController
  (return 0))