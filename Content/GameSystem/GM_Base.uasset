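; Base game mode that runs a timed round and sub-round progression for all players.
; LaunchRoundTimer collects round trackers until their count matches the player controllers, then loops, pushing round state to every tracker and waiting one round length.
; GoNextRound advances the sub-round, rolling into a new round when RoundTable's limit for the current round is exceeded.
; Counters freeze at the hardcoded final round, though the timer loop keeps running.
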(event Custom|LaunchRoundTimer
  (params (RoundTracker :type WB%20UI%20Manager%20Object%20Reference))
  (Utilities|Array|Add (Variables|Round|GetRoundTrackers) RoundTracker)
  (if (== (Utilities|Array|Length (Variables|Round|GetRoundTrackers)) (Class|GameplayStatics|GetNumPlayerControllers))
    (Default|MANAGENextRound (Variables|Round|GetRoundTrackers) (Variables|Round|GetRoundLength) (Variables|Round|GetCurrent%20Round) (Variables|Round|GetSub%20Round) (stale _neednewround__) :!label _label)
    (Utilities|FlowControl|RetriggerableDelay (Variables|Round|GetRoundLength))
    (bind _neednewround__ (CallFunction|GoNextRound))
    (goto _label)))

(fn ConstructionScript)

(fn GoNextRound
  ;[0 0 0 0.5 50] Check if max round is reached
  (if (not (and (>= (Variables|Round|GetSub%20Round) 7) (>= (Variables|Round|GetCurrent%20Round) 7)))
    (bind _output_get (LocalVariables|SetNeedNewRound (> (+ (Variables|Round|GetSub%20Round) 1) (.Value (Utilities|Map|Find (Variables|/Game/UI/Data/Rounds/D_Round.D_Round_C|GetRounds (Variables|Round|GetRoundTable)) (Variables|Round|GetCurrent%20Round))))))
    (if _output_get ; Pass to next round ?
      (Variables|Round|SetSub%20Round 1)
      (Variables|Round|SetCurrent%20Round (+ 1 (Variables|Round|GetCurrent%20Round)))
      (else
        (Variables|Round|SetSub%20Round (+ 1 (Variables|Round|GetSub%20Round)))))
    (return (LocalVariables|GetNeedNewRound))))