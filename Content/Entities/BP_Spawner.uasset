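; Enemy spawner actor that releases endless waves of BP_EnemyBase from BeginPlay.
; Each wave spawns one enemy per tick up to NumOfEnemy, randomly offset along world Y from the spawner's location.
; A message hands each new enemy's AI controller a reference to the level's BP_Base.
; After a short delay the counter resets and the loop repeats.
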(event EventBeginPlay
  (bind _returnvalue (Transformation|GetActorLocation))
  (bind _returnvalue_2 (Actor|GetActorOfClass "/Game/Entities/BP_Base.BP_Base_C"))
  (Variables|Default|SetBase _returnvalue_2)
  (if (< (Variables|Default|GetNewVar) (Variables|Default|GetNumOfEnemy)) :!label _label
    (Math|Integer|IncrementInt (Variables|Default|GetNewVar)
      (:%20%20
        (bind _returnvalue_3 (Game|SpawnActorfromClass "/Game/Entities/BP_EnemyBase.BP_EnemyBase_C" (Math|Conversions|ToTransform(Vector) (Math|Vector|MakeVector (+ (.x _returnvalue) 0.0) (+ (.y _returnvalue) (Math|Random|RandomFloatinRange -1e+03 1e+03)) (.z _returnvalue))) "AdjustIfPossibleButAlwaysSpawn" "MultiplyWithRoot" 0 0))
        (Class|BPIRunTree|GetObjectRef(Message) (AI|GetAIController _returnvalue_3) (Variables|Default|GetBase))
        (Utilities|FlowControl|DelayUntilNextTick)
        (goto _label)))
    (else
      (Utilities|FlowControl|Delay 5.0)
      (Variables|Default|SetNewVar 0)
      (goto _label))))

(fn ConstructionScript)