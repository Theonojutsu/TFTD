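; BP_Base is an actor that, once clicked, follows the mouse cursor at a raised height.
; The click stores a position 50 units above the actor, disables mesh physics simulation and opens a gate on Tick.
; Each tick then teleports it to the X and Y of a WorldDynamic hit under the cursor, keeping the stored Z.
; Nothing here closes the gate or restores physics.
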(event MouseInput|EventActorOnClicked
  (params (ButtonPressed :type Key%20Structure))
  (bind _returnvalue (Game|GetPlayerController 0))
  (bind _returnvalue_2 (Transformation|GetActorLocation))
  (bind _array (Utilities|Array|MakeArray "ObjectTypeQuery2"))
  (bind _hitresult (Class|PlayerController|GetHitResultUnderCursorforObjects _returnvalue _array false))
  (Variables|Default|SetLocation (Math|Vector|MakeVector (.x _returnvalue_2) (.y _returnvalue_2) (+ (.z _returnvalue_2) 5e+01)))
  (Physics|SetSimulatePhysics (Variables|Default|GetStaticMesh) false)
  (Utilities|FlowControl|Gate true) ; enters at Open
)

(event EventTick
  (params (DeltaSeconds :type Float%20%28single-precision%29))
  (bind _returnvalue (Game|GetPlayerController 0))
  (bind _array (Utilities|Array|MakeArray "ObjectTypeQuery2"))
  (bind _hitresult (Class|PlayerController|GetHitResultUnderCursorforObjects _returnvalue _array false))
  (Utilities|FlowControl|Gate true
    (:Exit
      (Transformation|SetActorLocation (Math|Vector|MakeVector (.x (.impactpoint _hitresult)) (.y (.impactpoint _hitresult)) (.z (Variables|Default|GetLocation))) false true))))

(fn ConstructionScript)